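; BP_SaveGame is a save game data container that holds the player's best score, level and material.
; Each variable has a plain getter and setter function that reads or overwrites it directly.
; It contains no validation, score comparison or disk read and write logic.
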(fn GetBestScore
  (return (Variables|Default|GetbestScore)))

(fn SetBestScore
  (params (bestScore :type Integer))
  (Variables|Default|SetbestScore bestScore))

(fn GetLevel
  (return (Variables|Default|Getlevel)))

(fn SetLevel
  (params (level :type Name))
  (Variables|Default|Setlevel level))

(fn GetMaterial
  (return (Variables|Default|Getmaterial)))

(fn SetMaterial
  (params (material :type Material%20Object%20Reference))
  (Variables|Default|Setmaterial material))