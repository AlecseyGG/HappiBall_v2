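; Player controller that shows the mouse cursor, holds the save game and lets the player trigger division of the level's happi balls.
; On BeginPlay it loads save slot "1" as BP_SaveGame and caches it, exposed through GetSave.
; The SearchBalls event caches every BP_BasePawn in the level.
; Pressing E calls DivisionHappiBall on each cached pawn and prints its name.
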(event Custom|SearchBalls
  (bind _outactors (Actor|GetAllActorsOfClass "/Game/Blueprint/Actor/BP_BasePawn.BP_BasePawn_C"))
  (Variables|Default|SetAllHappiBall_inLevel _outactors))

(event EventBeginPlay
  (Variables|Default|SetbShowMouseCursor true)
  (bind _returnvalue (SaveGame|LoadGamefromSlot "1"))
  (bind _asbp_save_game (Utilities|Casting|CastToBP_SaveGame _returnvalue))
  (Variables|Default|SetSave _asbp_save_game))

(event Input|KeyboardEvents|E
  (params (Key :type Key%20Structure :default "None"))
  (:Pressed
    (for _array_element (Variables|Default|GetAllHappiBall_inLevel)
      (Default|DivisionHappiBall _array_element)
      (Development|PrintString (Utilities|GetDisplayName _array_element)))))

(event Input|KeyboardEvents|Q
  (params (Key :type Key%20Structure :default "None")))

(event Input|KeyboardEvents|A
  (params (Key :type Key%20Structure :default "None")))

(event Input|KeyboardEvents|D
  (params (Key :type Key%20Structure :default "None")))

(fn ConstructionScript)

(fn GetSave
  (return (Variables|Default|GetSave)))