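; Base pawn for a physics-driven "Happi" ball that is pushed along X every tick, shifts sideways and can split or merge.
; It registers with the player controller, takes its material from the save and reports distance to a Block end point.
; DivisionHappiBall spawns small balls with inherited impulse.
; A timeline lerps non-root balls to the root until radii overlap, adding their count to step up its size and mass.
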(event Custom|MovingRigt
  (params (New%20Location%20Y :type Float%20%28single-precision%29))
  ;[1 1 1] MovingLeftAndRight
  (Transformation|AddWorldOffset (Variables|Default|GetSphereMesh) (Math|Vector|MakeVector 0.0 New%20Location%20Y 0.0) false false))

(event Custom|MovingLeft
  (params (New%20Location%20Y :type Float%20%28single-precision%29))
  ;[1 1 1] MovingLeftAndRight
  (Transformation|AddWorldOffset (Variables|Default|GetSphereMesh) (Math|Vector|MakeVector 0.0 New%20Location%20Y 0.0) false false))

(event Custom|StopToMoveRootBall
  (bind _rootball (Variables|Default|GetrootBall))
  ;[1 1 1] Move to root ball
  (bind _alpha (Timeline|MoveToRoot Stop)
    (:Update
      (bind (_returnvalue _locationrootball _selflocation) (CallFunction|GettingDrivingDirection (Variables|Default|GetrootBall)))
      (if _returnvalue
        ;[0.4163 1 0.4632] combine balls
        (bind _result (CallFunction|AddHappiBalls _rootball (Variables|Default|GetAmmountHappiBalls)))
        (CallFunction|TransformScaleHappiBall _rootball _result)
        (CallFunction|DestroySelf)
        (else
          ;[1 0.2969 0.2969] TransformLocation
          (Transformation|SetActorLocation (Math|Vector|Lerp(Vector) _selflocation _locationrootball _alpha) false false))))))

(event Custom|MoveToRootBall
  (params (RootBall :type BP%20Base%20Pawn%20Object%20Reference))
  ;[1 1 1] Move to root ball
  (if (not (Variables|Default|GetIRootBall?))
    (Variables|Default|SetrootBall RootBall)
    (bind _alpha (Timeline|MoveToRoot Play)
      (:Update
        (bind (_returnvalue _locationrootball _selflocation) (CallFunction|GettingDrivingDirection (Variables|Default|GetrootBall)))
        (if _returnvalue
          ;[0.4163 1 0.4632] combine balls
          (bind _result (CallFunction|AddHappiBalls (Variables|Default|GetrootBall) (Variables|Default|GetAmmountHappiBalls)))
          (CallFunction|TransformScaleHappiBall (Variables|Default|GetrootBall) _result)
          (CallFunction|DestroySelf)
          (else
            ;[1 0.2969 0.2969] TransformLocation
            (Transformation|SetActorLocation (Math|Vector|Lerp(Vector) _selflocation _locationrootball _alpha) false false)))))))

(event EventBeginPlay
  (bind _asbp_player_controller (Utilities|Casting|CastToBP_PlayerController (Game|GetPlayerController 0)))
  (Variables|Default|SetPlayerController _asbp_player_controller)
  (bind _returnvalue (Actor|GetActorOfClass "/Game/Blueprint/Actor/NewFolder/Block.Block_C"))
  (Variables|Default|SetendPoint _returnvalue)
  (Default|AddHappiBall (Variables|Default|GetPlayerController) self)
  (Utilities|FlowControl|Delay 0.05)
  (bind _save (Default|GetSave (Variables|Default|GetPlayerController)))
  (Rendering|Material|SetMaterial (Variables|Default|GetSphereMesh) 0 (Default|GetMaterial _save)))

(event EventTick
  (params (DeltaSeconds :type Float%20%28single-precision%29))
  ;[1 1 1] Print Speed and Mass
  (Physics|AddForce (Variables|Default|GetSphereMesh) "10000.000000, 0, 0" "None" false))

(fn ConstructionScript)

(fn DivisionHappiBall
  (bind _minammounthappiball (LocalVariables|GetMinAmmountHappiBall))
  (bind _spheremesh (Variables|Default|GetSphereMesh))
  (for _index (range 0 (- (Variables|Default|GetAmmountHappiBalls) 2))
    (bind _returnvalue (Game|SpawnActorfromClass (LocalVariables|GetEmergingBall) (Math|Transform|MakeTransform (+ (Transformation|GetWorldLocation (Variables|Default|GetSphereMesh self)) (Math|Random|RandomUnitVector)) "0, 0, 0" (LocalVariables|GetSmallSizeBall)) "AdjustIfPossibleButAlwaysSpawn" 0 _minammounthappiball 0))
    (Transformation|SetWorldScale3D _spheremesh "0.250000,0.250000,0.250000")
    (Class|PrimitiveComponent|SetMassScale _spheremesh "None" (Physics|GetMass _spheremesh))
    (Physics|AddImpulse (Variables|BP_BasePawn_C|GetSphereMesh _returnvalue) (Transformation|GetVelocity self) "None" false))
  (Variables|Default|SetAmmountHappiBalls _minammounthappiball))

(fn DistancetoEndPoint
  (return (Transformation|GetDistanceTo (Variables|Default|GetendPoint))))

(fn SetRootBall
  (params (IRootBall? :type Boolean))
  (Variables|Default|SetIRootBall? IRootBall?))

(fn GettingDrivingDirection
  (params (rootBall :type BP%20Base%20Pawn%20Object%20Reference))
  (bind _sphere (Variables|Default|GetSphere))
  (bind _sphere_2 (Variables|BP_BasePawn_C|GetSphere rootBall))
  (bind _returnvalue (Transformation|GetWorldLocation _sphere))
  (bind _returnvalue_2 (Transformation|GetWorldLocation _sphere_2))
  (return (> (+ (+ (Components|Sphere|GetScaledSphereRadius (Variables|BP_BasePawn_C|GetSphere rootBall)) (Components|Sphere|GetScaledSphereRadius (Variables|Default|GetSphere))) (LocalVariables|GetacceptableError)) (Math|Vector|Distance(Vector) _returnvalue _returnvalue_2)) _returnvalue_2 _returnvalue))

(fn AddHappiBalls
  (params (ammountHappiBall :type Integer))
  (bind _output_get (Variables|Default|SetAmmountHappiBalls (+ ammountHappiBall (Variables|Default|GetAmmountHappiBalls))))
  (return _output_get))

(fn TransformScaleHappiBall
  (params (NewParam :type Integer))
  (if (> NewParam 4)
    (if (not (LocalVariables|GetIBigSize?))
      (Transformation|SetWorldScale3D (Variables|Default|GetSphereMesh) (LocalVariables|GetbigSize))
      (LocalVariables|SetIBigSize? true)
      (Class|PrimitiveComponent|SetMassScale (Variables|Default|GetSphereMesh) "None" 5e+01 :!label _label))
    (elif (> NewParam 1)
      (if (not (LocalVariables|GetIMiddleSize?))
        (Transformation|SetWorldScale3D (Variables|Default|GetSphereMesh) (LocalVariables|GetmidSize))
        (LocalVariables|SetIMiddleSize? true)
        (goto _label)))))

(fn GetIRootBall
  (return (Variables|Default|GetIRootBall?)))

(fn DestroySelf
  (Default|RemoveHappiBall (Variables|Default|GetPlayerController) self)
  (Actor|DestroyActor))